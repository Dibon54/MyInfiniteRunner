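; Magnet power-up pickup that temporarily sets MagnetActive on the main character when it overlaps the pickup's box.
; On overlap it hides itself, disables collision and adds a MagnetTimer_HUD widget to the viewport.
; The hidden actor stays alive through a ten-second Delay, then clears the flag and destroys itself, printing debug messages on activation and expiry.
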(event `self.ReceiveActorBeginOverlap`
  (params (OtherActor :type "Actor Object Reference")))

(event `self.Box.OnComponentBeginOverlap`
  (params (OverlappedComponent :type "PrimitiveComponent Object Reference") (OtherActor :type "Actor Object Reference") (OtherComp :type "PrimitiveComponent Object Reference") (OtherBodyIndex :type Integer) (bFromSweep :type Boolean) (SweepResult :type "HitResult Structure (by ref)"))
  (bind _asmain_charachter_bp (cast `/Game/Blueprints/Normal_BP/MainCharachter_BP` OtherActor))
  (set `/Game/Blueprints/Normal_BP/MainCharachter_BP.MagnetActive` true _asmain_charachter_bp)
  (`KismetSystemLibrary.PrintString` "Magnet active")
  (`SceneComponent.SetVisibility` (`self.DefaultSceneRoot`) false true)
  (`self.SetActorEnableCollision` false)
  (bind _returnvalue (`|CreateWidget` "/Game/Blueprints/UI/MagnetTimer_HUD.MagnetTimer_HUD_C"))
  (`UserWidget.AddToViewport` _returnvalue 0)
  (`KismetSystemLibrary.Delay` 10.0)
  (set `/Game/Blueprints/Normal_BP/MainCharachter_BP.MagnetActive` false _asmain_charachter_bp)
  (`KismetSystemLibrary.PrintString` "MAgnet inactive")
  (`self.K2_DestroyActor`))

(fn `UserConstructionScript`)