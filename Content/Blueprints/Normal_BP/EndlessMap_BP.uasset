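; EndlessMap_BP is an endless-runner map segment that fills itself with obstacles and coins and chains the next segment.
; On BeginPlay it builds a lane grid, keeps points whose downward trace hits, then randomly places child-actor obstacles or Coin_BP at shuffled points.
; When the player overlaps Box, it spawns the next segment at ArrowEnd, raises walk speed within limits and destroys itself after a delay.
; Overlapping BoxColFall calls the player's Death.
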(event `self.ReceiveBeginPlay`
  ;[1 1 1] Obstacle spawn point and spawn functions
  (`self.initSpawnPoints`)
  (`self.SpawnObstacles`))

(event `self.Box.OnComponentBeginOverlap`
  (params (OverlappedComponent :type "PrimitiveComponent Object Reference") (OtherActor :type "Actor Object Reference") (OtherComp :type "PrimitiveComponent Object Reference") (OtherBodyIndex :type Integer) (bFromSweep :type Boolean) (SweepResult :type "HitResult Structure (by ref)"))
  ;[1 1 1] PlatformSpawner
  (cast `/Game/Blueprints/Normal_BP/MainCharachter_BP` OtherActor)
  (`|SpawnActorFromClass` "EndlessMap_BP_C" (`SceneComponent.K2_GetComponentToWorld` (`self.ArrowEnd`)) "Undefined" "OverrideRootScale" null null)
  (bind _asmain_charachter_bp (cast `/Game/Blueprints/Normal_BP/MainCharachter_BP` (`GameplayStatics.GetPlayerCharacter` 0)))
  (bind _charactermovement (`Character.CharacterMovement` _asmain_charachter_bp))
  (set `CharacterMovementComponent.MaxWalkSpeed` (`KismetMathLibrary.FClamp` (* (`CharacterMovementComponent.MaxWalkSpeed` _charactermovement) 1.02) 1200.0 2400.0) _charactermovement)
  (`KismetSystemLibrary.Delay` 10.0)
  (`self.K2_DestroyActor`))

(event `self.BoxColFall.OnComponentBeginOverlap`
  (params (OverlappedComponent :type "PrimitiveComponent Object Reference") (OtherActor :type "Actor Object Reference") (OtherComp :type "PrimitiveComponent Object Reference") (OtherBodyIndex :type Integer) (bFromSweep :type Boolean) (SweepResult :type "HitResult Structure (by ref)"))
  ;[1 1 1] Play death event if player falls
  (bind _asmain_charachter_bp (cast `/Game/Blueprints/Normal_BP/MainCharachter_BP` OtherActor))
  (`/Game/Blueprints/Normal_BP/MainCharachter_BP.Death` _asmain_charachter_bp))

(fn `initSpawnPoints`
  (locals (pendingTransform :type "Transform Structure"))
  (bind _returnvalue_x (`KismetMathLibrary.BreakVector` (`self.K2_GetActorLocation`)))
  (bind _pendingtransform_location (`KismetMathLibrary.BreakTransform` (`local.pendingTransform`)))
  (for _array_element (`self.LanePositions`)
    (for _index (range 5)
      (bind _output_get (set `local.pendingTransform` (`KismetMathLibrary.MakeTransform` (`KismetMathLibrary.MakeVector` (+ _returnvalue_x (`KismetMathLibrary.Conv_IntToDouble` (* _index 1000))) _array_element -220.0))))
      ;[1 1 1] Trace spawnpoint, never spawn in the air
      (bind (_outhit _returnvalue) (`KismetSystemLibrary.LineTraceSingle` :`Start` (+ _pendingtransform_location (0.0 0.0 500.0)) :`End` (+ _pendingtransform_location (0.0 0.0 -1000.0)) :`TraceChannel` "TraceTypeQuery1" :`bIgnoreSelf` false :`DrawTime` 100.0))
      (if _returnvalue
        (`KismetArrayLibrary.Array_Add` (`self.SpawnPoints`) _output_get)))))

(fn `SpawnObstacles`
  (locals (RandomSpawnPoints :type "Array of Transform Structure"))
  (bind _randomspawnpoints (`local.RandomSpawnPoints`))
  (bind _output_get (set `local.RandomSpawnPoints` (`self.SpawnPoints`)))
  (`KismetArrayLibrary.Array_Shuffle` _output_get)
  (for _index (range (+ (`KismetMathLibrary.RandomIntegerInRange` 3 5) 1))
    (if (not (<= (`KismetArrayLibrary.Array_Length` _randomspawnpoints) _index))
      (switch `int` (`KismetMathLibrary.RandomIntegerInRange` 0 3)
        (:`0`
          (bind _output_location (`KismetMathLibrary.BreakTransform` (`|GetArrayItem` _randomspawnpoints _index)))
          (bind _returnvalue (`KismetMathLibrary.InverseTransformLocation` (`self.GetTransform`) _output_location))
          (`AddComponent|NODE_AddChildActorComponent-0` :`RelativeTransform` (`KismetMathLibrary.Conv_VectorToTransform` _returnvalue)))
        (:`1`
          (`|SpawnActorFromClass` "/Game/Materials/Coin_BP.Coin_BP_C" (`KismetMathLibrary.Conv_VectorToTransform` _output_location) "Undefined" "OverrideRootScale" null null))
        (:`2`
          (`AddComponent|NODE_AddChildActorComponent-3` :`RelativeTransform` (`KismetMathLibrary.Conv_VectorToTransform` _returnvalue)))
        (:`3`
          (`AddComponent|NODE_AddChildActorComponent-1` :`RelativeTransform` (`KismetMathLibrary.Conv_VectorToTransform` _returnvalue)))))))

(fn `UserConstructionScript`)