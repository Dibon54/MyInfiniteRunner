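; Player character Blueprint for an endless-runner style game, pushed forward along world X every tick at a Speed-scaled input.
; Input adds sideways steering from control yaw, a jump that raises an IsJumping flag for half a second, and a crouch that shrinks the whole actor.
; BeginPlay shows the score HUD; Death turns the mesh into a ragdoll, clears widgets and opens the game over screen with a cursor.
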(event `Death`
  (bind _mesh (`self.Mesh`))
  ;[0.5706 1 0.06157] Death animation + game paused + game over screen
  (`CharacterMovementComponent.DisableMovement` (`self.CharacterMovement`))
  (`PrimitiveComponent.SetCollisionEnabled` _mesh "QueryAndPhysics")
  (`SkeletalMeshComponent.SetAllBodiesSimulatePhysics` _mesh true)
  (`SkeletalMeshComponent.SetAllBodiesPhysicsBlendWeight` _mesh 1.0 false)
  (`WidgetLayoutLibrary.RemoveAllWidgets`)
  (bind _returnvalue (`|CreateWidget` "/Game/Blueprints/UI/GameOver.GameOver_C"))
  (`UserWidget.AddToViewport` _returnvalue 0)
  (set `PlayerController.bShowMouseCursor` true (`GameplayStatics.GetPlayerController` 0)))

(event `InputAction|JumpAction`
  (params (Key :type "Key Structure"))
  ;[1 0 0.171] Movement
  (:`Pressed`
    (`self.Jump`)
    (set `self.IsJumping` true)
    (`KismetSystemLibrary.Delay` 0.5)
    (set `self.IsJumping` false)))

(event `InputAxis|Move Right/Left`
  (params (AxisValue :type "Float (single-precision)"))
  ;[1 0 0.171] Movement
  (`self.AddMovementInput` (`KismetMathLibrary.GetRightVector` (`KismetMathLibrary.MakeRotator` 0.0 0.0 (.yaw (`self.GetControlRotation`)))) AxisValue))

(event `InputAction|Crouch`
  (params (Key :type "Key Structure"))
  ;[1 0 0.171] Movement
  (:`Pressed`
    (`self.SetActorRelativeScale3D` (0.15 0.15 0.15)))
  (:`Released`
    (`self.SetActorRelativeScale3D` (1.0 1.0 1.0))))

(event `self.ReceiveTick`
  (params (DeltaSeconds :type "Float (single-precision)"))
  ;[1 1 1] Constantly running forward
  (`self.AddMovementInput` (1.0 0.0 0.0) (`self.Speed`)))

(event `self.ReceiveBeginPlay`
  ;[1 1 1] Showing score top left
  (bind _returnvalue (`|CreateWidget` "/Game/Blueprints/UI/Score_HUD.Score_HUD_C"))
  (`UserWidget.AddToViewport` _returnvalue 0))

(fn `UserConstructionScript`)