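; Player character for an auto-running game, pushed along world X every tick by Speed while the player steers sideways and jumps.
; Crouch shrinks the whole actor while held, and Death disables movement and ragdolls the mesh.
; BeginPlay shows the score HUD.
; The S key pauses the game, then a FlipFlop alternates between showing the EndGame widget with cursor and removing all widgets, without unpausing.
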(event `Death`
  (bind _mesh (`self.Mesh`))
  (`CharacterMovementComponent.DisableMovement` (`self.CharacterMovement`))
  (`PrimitiveComponent.SetCollisionEnabled` _mesh "QueryAndPhysics")
  (`SkeletalMeshComponent.SetAllBodiesSimulatePhysics` _mesh true)
  (`SkeletalMeshComponent.SetAllBodiesPhysicsBlendWeight` _mesh 1.0 false))

(event `InputAction|JumpAction`
  (params (Key :type "Key Structure"))
  ;[1 1 1] Movement
  (:`Pressed`
    (`self.Jump`)
    (set `self.IsJumping` true)
    (`KismetSystemLibrary.Delay` 0.5)
    (set `self.IsJumping` false)))

(event `InputAxis|Move Right/Left`
  (params (AxisValue :type "Float (single-precision)"))
  ;[1 1 1] Movement
  (`self.AddMovementInput` (`KismetMathLibrary.GetRightVector` (`KismetMathLibrary.MakeRotator` 0.0 0.0 (.yaw (`self.GetControlRotation`)))) AxisValue))

(event `InputAction|Crouch`
  (params (Key :type "Key Structure"))
  ;[1 1 1] Movement
  (:`Pressed`
    (`self.SetActorRelativeScale3D` (0.15 0.15 0.15)))
  (:`Released`
    (`self.SetActorRelativeScale3D` (1.0 1.0 1.0))))

(event `self.ReceiveTick`
  (params (DeltaSeconds :type "Float (single-precision)"))
  (`self.AddMovementInput` (1.0 0.0 0.0) (`self.Speed`)))

(event `self.ReceiveBeginPlay`
  (bind _returnvalue (`|CreateWidget` "/Game/Blueprints/Score_HUD.Score_HUD_C"))
  (`UserWidget.AddToViewport` _returnvalue 0))

(event `Key|S`
  (params (Key :type "Key Structure"))
  (bind _returnvalue (`GameplayStatics.GetPlayerController` 0))
  (:`Pressed`
    (`GameplayStatics.SetGamePaused` true)
    (`/Engine/EditorBlueprintResources/StandardMacros.FlipFlop`
      (:`A`
        (bind _returnvalue_2 (`|CreateWidget` "/Game/Blueprints/EndGame.EndGame_C"))
        (`UserWidget.AddToViewport` _returnvalue_2 0)
        (set `PlayerController.bShowMouseCursor` true _returnvalue))
      (:`B`
        (`WidgetLayoutLibrary.RemoveAllWidgets`)
        (set `PlayerController.bShowMouseCursor` false _returnvalue)))))

(fn `UserConstructionScript`)