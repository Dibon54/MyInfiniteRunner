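; EndlessMap_BP is a map segment for an endless runner that fills its lanes with random obstacles.
; Its construction script builds a grid of arrow-based spawn points along each lane, shuffles them and attaches child actors at a random number of them, choosing between two branches.
; When MainCharachter_BP overlaps the Box, it spawns an actor at ArrowEnd to continue the map, then destroys itself after a delay.
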(event `self.Box.OnComponentBeginOverlap`
  (params (OverlappedComponent :type "PrimitiveComponent Object Reference") (OtherActor :type "Actor Object Reference") (OtherComp :type "PrimitiveComponent Object Reference") (OtherBodyIndex :type Integer) (bFromSweep :type Boolean) (SweepResult :type "HitResult Structure (by ref)"))
  ;[1 1 1] PlatformSpawner
  (cast `/Game/Blueprints/MainCharachter_BP` OtherActor)
  (`|SpawnActorFromClass` "EndlessMap_BP_C" (`SceneComponent.K2_GetComponentToWorld` (`self.ArrowEnd`)) "Undefined" "OverrideRootScale" null null)
  (`KismetSystemLibrary.Delay` 10.0)
  (`self.K2_DestroyActor`))

(fn `initSpawnPoints`
  (for _array_element (`self.LanePositions`)
    (for _index (range 5)
      (bind _returnvalue (`AddComponent|NODE_AddArrowComponent-0` :`RelativeTransform` (`KismetMathLibrary.MakeTransform` (`KismetMathLibrary.MakeVector` (`KismetMathLibrary.Conv_IntToDouble` (* _index 1000)) _array_element))))
      (`KismetArrayLibrary.Array_Add` (`self.SpawnPoints`) (`SceneComponent.K2_GetComponentToWorld` _returnvalue)))))

(fn `SpawnObstacles`
  (locals (RandomSpawnPoints :type "Array of Transform Structure"))
  (bind _output_get (set `local.RandomSpawnPoints` (`self.SpawnPoints`)))
  (`KismetArrayLibrary.Array_Shuffle` _output_get)
  (for _index (range (+ (`KismetMathLibrary.RandomIntegerInRange` 4 10) 1))
    (switch `int` (`KismetMathLibrary.RandomIntegerInRange` 0 1)
      (:`0`
        (bind _returnvalue (`KismetMathLibrary.MakeRelativeTransform` (`|GetArrayItem` (`local.RandomSpawnPoints`) _index) (`self.GetTransform`)))
        (`AddComponent|NODE_AddChildActorComponent-0` :`RelativeTransform` _returnvalue))
      (:`1`
        (`AddComponent|NODE_AddChildActorComponent-1` :`RelativeTransform` _returnvalue)))))

(fn `UserConstructionScript`
  (`self.initSpawnPoints`)
  (`self.SpawnObstacles`))